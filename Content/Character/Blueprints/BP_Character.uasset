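; BP_Character is a player-controlled character Blueprint that handles basic movement and mouse look.
; MoveForward and MoveRight axis inputs add movement along the control rotation's forward and right vectors, scaled by MoveSpeed.
; LookUp and LookAround feed controller pitch and yaw, which steer that movement direction.
; The forward vector uses the full control rotation, pitch included, and the construction script is empty.
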(event Input|AxisEvents|InputAxisMoveForward
  (params (AxisValue :type Float%20%28single-precision%29))
  ;[0 0 0] Move
  (Pawn|Input|AddMovementInput (Math|Vector|GetForwardVector (Pawn|GetControlRotation :!class /Script/Engine.Pawn)) (* AxisValue (Variables|Default|GetMoveSpeed)) false))

(event Input|AxisEvents|InputAxisMoveRight
  (params (AxisValue :type Float%20%28single-precision%29))
  ;[0 0 0] Move
  (Pawn|Input|AddMovementInput (Math|Vector|GetRightVector (Pawn|GetControlRotation :!class /Script/Engine.Pawn)) (* AxisValue (Variables|Default|GetMoveSpeed)) false))

(event Input|AxisEvents|InputAxisLookUp
  (params (AxisValue :type Float%20%28single-precision%29))
  ;[0 0 0] MouseLook
  (Pawn|Input|AddControllerPitchInput AxisValue))

(event Input|AxisEvents|InputAxisLookAround
  (params (AxisValue :type Float%20%28single-precision%29))
  ;[0 0 0] MouseLook
  (Pawn|Input|AddControllerYawInput AxisValue))

(fn ConstructionScript)